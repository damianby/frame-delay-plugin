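; Composure media plate element that can delay its media input by a set number of frames before compositing.
; A frame delayer, created at construction or BeginPlay, replaces the registered input when the delay is nonzero.
; The plate passes through ProcessPlateForKeying, currently a pass-through hook, and registers separately as ProcessedPlate to protect frozen inputs.
; Parent transform passes then run, with editor color picking wired to the plate and keyer result.
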(event EventBeginPlay
  (CallFunction|InitializeFrameRetarder))

(event Collision|EventActorBeginOverlap
  (params (OtherActor :type Actor%20Object%20Reference)))

(event EventTick
  (params (DeltaSeconds :type Float%20%28single-precision%29)))

(fn ConstructionScript
  (CallFunction|InitializeFrameRetarder))

(fn RenderCompElement
  (params (bCameraCutThisFrame :type Boolean))
  ;[1 1 1] 1) Get the media input texture and delay if needed
  (bind (_passresult _returnvalue) (Class|CompositingElement|FindInputPass "/Script/Composure.CompositingMediaInput" "None"))
  (Utilities|IsValid _passresult
    (:Is%20Valid
      (Class|FrameDelayer|FeedTexture (Variables|Default|GetFrameDelayer) _passresult)
      (Class|CompositingElement|RegisterPassResult (Variables|/Script/Composure.CompositingElementPass|GetPassName _returnvalue) (select (Math|Conversions|ToBoolean(Integer) (Variables|FrameDelay|GetNum%20Frames)) (Variables|Default|GetOutputTexture) _passresult) true) ; Overwrite input so we can use delayed everywhere
      ;[0.6038 0.6038 1] 2) Apply optional color correction
      (bind _processedplate (CallFunction|ProcessPlateforKeying (select (Math|Conversions|ToBoolean(Integer) (Variables|FrameDelay|GetNum%20Frames)) (Variables|Default|GetOutputTexture) _passresult)))
      (bind _output_get (LocalVariables|SetMediaInputResult _processedplate))
      (Class|CompositingElement|RegisterPassResult "ProcessedPlate" _output_get true) ; DO NOT set this to overwrite the the input -\nWe could freeze inputs, and this is not an input,\nwe don't want to overwrite it when frozen.
    )
    (:Is%20Not%20Valid
      (bind _processedplate_2 (CallFunction|ProcessPlateforKeying (Class|CompositingElement|GetLatestRenderResult)))
      (LocalVariables|SetMediaInputResult _processedplate_2)))
  ;[0.3185 0.3185 1] 3) Set as chroma color picking target
  (bind _astexture_render_target_2d (Utilities|Casting|CastToTextureRenderTarget2D (LocalVariables|GetMediaInputResult))
    (:then
      (Class|CompositingElement|SetEditorColorPickingTarget _astexture_render_target_2d))
    (:CastFailed
      _))
  ;[0.1329 0.1329 1] 4) Apply transform passes (keying, etc.)
  (bind _returnvalue_2 (|CallParentFunction bCameraCutThisFrame))
  (LocalVariables|SetInternalPipelineResult _returnvalue_2)
  ;[0.03311 0.03311 1] 5) Find chroma keying result
  (bind _passresult_2 (Class|CompositingElement|FindTransformPass "/Script/Composure.MultiPassChromaKeyer" "None"))
  (Utilities|IsValid _passresult_2
    (:Is%20Valid
      ;[0 0 1] 6) Set color picker result image
      (Class|CompositingElement|SetEditorColorPickerDisplayImage _passresult_2))
    (:Is%20Not%20Valid
      (Class|CompositingElement|SetEditorColorPickerDisplayImage (LocalVariables|GetInternalPipelineResult))))
  (return (LocalVariables|GetInternalPipelineResult)))

(fn ProcessPlateforKeying
  (params (RawMediaPlate :type Texture%20Object%20Reference))
  (return RawMediaPlate))

(fn InitializeFrameRetarder
  (Utilities|IsValid (Variables|Default|GetFrameDelayer)
    (:Is%20Valid
      (bind _returnvalue (Class|FrameDelayer|IsInitialized (Variables|Default|GetFrameDelayer)))
      (if (not _returnvalue)
        (bind _outtexture (Class|FrameDelayer|Initialize (Variables|Default|GetFrameDelayer) (Variables|FrameDelay|GetNum%20Frames)))
        (Variables|Default|SetOutputTexture _outtexture)))
    (:Is%20Not%20Valid
      (bind (_framedelayer _outtexture_2) (Class|TextureUtilitiesBPLibrary|CreateFrameDelayer (Variables|FrameDelay|GetNum%20Frames)))
      (Variables|Default|SetFrameDelayer _framedelayer)
      (Variables|Default|SetOutputTexture _outtexture_2))))